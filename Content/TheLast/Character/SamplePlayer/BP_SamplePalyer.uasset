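; Sample player character Blueprint that equips a twin-blade melee weapon when play begins.
; BeginPlay runs the parent logic, spawns BPW_TwinBlade at the left weapon socket and registers it as the current melee weapon through the combat component.
; On success, the weapon's left and right components snap separately to the matching mesh sockets, so one weapon actor covers both hands.
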(event EventBeginPlay
  (bind _self self)
  (bind _mesh (Variables|Character|GetMesh))
  (|CallParentFunction)
  (bind _returnvalue (Game|SpawnActorfromClass "/Game/TheLast/Weapon/BPW_TwinBlade.BPW_TwinBlade_C" (Transformation|GetSocketTransform (Variables|Character|GetMesh) "Weapon_L" "RTS_World") "Undefined" _self _self))
  (bind _returnvalue_2 (Class|TLCombatComponent|SetCurrentWeaponOfType (Variables|Default|GetBP_TL_CombatComponent) "E_MELEE" _returnvalue))
  (if _returnvalue_2
    (Transformation|AttachComponentToComponent (Variables|/Game/TheLast/Weapon/BPW_TwinBlade.BPW_TwinBlade_C|GetWeapon_L _returnvalue) _mesh "Weapon_L" "SnapToTarget" "SnapToTarget" "KeepRelative" true)
    (Transformation|AttachComponentToComponent (Variables|/Game/TheLast/Weapon/BPW_TwinBlade.BPW_TwinBlade_C|GetWeapon_R _returnvalue) _mesh "Weapon_R" "SnapToTarget" "SnapToTarget" "KeepRelative" true)))

(fn ConstructionScript
  (|CallParentFunction))