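; Combat component for the sample player character that plays montages and finds enemies inside melee-style hit volumes.
; On BeginPlay it caches the player, then calls AttackEnter after a fixed delay.
; CharacterPlayMontage plays on the player's mesh and calls MotionEnd on completion or blend-out.
; Box and sphere checks spawn damage-volume actors, query ahead of the owner, and return unique characters matching EnemyObjectTypes.
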(event EventBeginPlay
  (|CallParentFunction)
  (bind _asbp_sample_palyer (Utilities|Casting|CastToBP_SamplePalyer (Variables|Default|GetPlayerCharacter)))
  (bind _output_get (Variables|Default|SetPlayer _asbp_sample_palyer))
  (Utilities|FlowControl|Delay 1e+01)
  (Class|TLCombatComponent|AttackEnter))

(event EventCharacterPlayMontage
  (params (MontageToPlay :type Anim%20Montage%20Object%20Reference) (PlayRate :type Float%20%28single-precision%29) (StartSection :type Name :default "None") (StartingPos :type Float%20%28single-precision%29))
  (Utilities|IsValid MontageToPlay
    (:Is%20Valid
      (Animation|Montage|PlayMontage (Variables|/Script/Engine.Character|GetMesh (Variables|Default|GetPlayer)) 0 PlayRate StartingPos StartSection
        (:OnCompleted
          _)
        (:OnBlendOut
          _))
      (Class|TLCombatComponent|MotionEnd))
    (:Is%20Not%20Valid
      (Development|PrintString "CombatComponnet  ERROR: No Valid Montage To Play" true true "(R=0.671875,G=0.000000,B=0.010183,A=1.000000)" 5.0))))

(fn TLBoxCheck
  (params (FwdLocationOffset :type Float%20%28single-precision%29) (NewScale :type Vector :default "0, 0, 0") (bFalseFaceAttacker :type Boolean))
  (bind _returnvalue (Components|GetOwner))
  (bind _returnvalue_2 (Transformation|GetActorLocation _returnvalue))
  (Utilities|Array|Clear (Variables|Default|GetOut))
  (bind _returnvalue_3 (Game|SpawnActorfromClass "/Game/TheLast/DamageCollision/BP_BaseDamageBox.BP_BaseDamageBox_C" (Math|Transform|MakeTransform _returnvalue_2 (Math|Rotator|MakeRotator 0.0 0.0 (.Yaw (Math|Rotator|BreakRotator (Transformation|GetActorRotation _returnvalue)))) "1,1,1") "Undefined" 0 self))
  (bind _returnvalue_4 (Class|BaseDamageBox|BoxCheck _returnvalue_3 _returnvalue_2 (* (Math|Vector|Normalize (Transformation|GetActorForwardVector _returnvalue)) FwdLocationOffset) NewScale "/Script/Engine.Actor"))
  (for _array_element _returnvalue_4
    (bind _asbp_char_base (Utilities|Casting|CastToBP_CharBase _array_element))
    (bind _array_element_2 (Utilities|Array|ForEachLoopwithBreak (Variables|Default|GetEnemyObjectTypes) :!label _label)
      (:LoopBody
        (if (Utilities|Enum|Equal(Enum) (Variables|/Game/TheLast/Character/BaseChar/BP_CharBase.BP_CharBase_C|GetSelfObjectType _asbp_char_base) _array_element_2)
          (Utilities|Array|AddUnique (Variables|Default|GetOut) _array_element)
          (goto _label Break)))))
  (return (Variables|Default|GetOut)))

(fn TLSphereCheck
  (params (FwdLocationOffset :type Float%20%28single-precision%29) (NewScale :type Vector :default "0, 0, 0") (bFalseFaceAttacker :type Boolean))
  (bind _returnvalue (Components|GetOwner))
  (bind _returnvalue_2 (Transformation|GetActorLocation _returnvalue))
  (Utilities|Array|Clear (Variables|Default|GetOut))
  (bind _returnvalue_3 (Game|SpawnActorfromClass "/Game/TheLast/DamageCollision/BP_BaseDamageSphere.BP_BaseDamageSphere_C" (Math|Transform|MakeTransform _returnvalue_2 (Math|Rotator|MakeRotator 0.0 0.0 (.Yaw (Math|Rotator|BreakRotator (Transformation|GetActorRotation _returnvalue)))) "1,1,1") "Undefined" 0 self))
  (bind _returnvalue_4 (Class|BaseDamageSphere|SphereCheck _returnvalue_3 _returnvalue_2 (* (Math|Vector|Normalize (Transformation|GetActorForwardVector _returnvalue)) FwdLocationOffset) NewScale "/Script/Engine.Actor"))
  (for _array_element _returnvalue_4
    (bind _asbp_char_base (Utilities|Casting|CastToBP_CharBase _array_element))
    (bind _array_element_2 (Utilities|Array|ForEachLoopwithBreak (Variables|Default|GetEnemyObjectTypes) :!label _label)
      (:LoopBody
        (if (Utilities|Enum|Equal(Enum) (Variables|/Game/TheLast/Character/BaseChar/BP_CharBase.BP_CharBase_C|GetSelfObjectType _asbp_char_base) _array_element_2)
          (Utilities|Array|AddUnique (Variables|Default|GetOut) _array_element)
          (goto _label Break)))))
  (return (Variables|Default|GetOut)))